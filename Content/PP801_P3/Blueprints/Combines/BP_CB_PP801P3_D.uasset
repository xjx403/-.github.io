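; Player character Blueprint handling keyboard and mouse input for weapons, combat and movement.
; X cycles the anim Blueprint's 状态 state through unarmed, gun and knife, spawning, socket-attaching and destroying weapon actors.
; Left click fires the gun or plays a melee montage by state; Shift and Ctrl handle running and crouch toggling.
; E reloads ammo via montage; a second E handler is an attack template checking separate weapon flags, with some montages unset.
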(event `self.ReceiveBeginPlay`
  ;[1 1 1] 注释
  (bind _asnew_man_anim_bp1 (cast `/Game/PP801_P3/Animations/Characters/NewAnimaBP/newMan_AnimBP1` (`SkeletalMeshComponent.GetAnimInstance` (`self.Mesh`))))
  (set `self.As New Man Anim BP1_0` _asnew_man_anim_bp1))

(event `Key|X`
  (params (Key :type "Key Structure"))
  (bind _as_new_man_anim_bp1_0 (`self.As New Man Anim BP1_0`))
  (bind `_状态` (`/Game/PP801_P3/Animations/Characters/NewAnimaBP/newMan_AnimBP1.状态` (`self.As New Man Anim BP1_0`)))
  ;[1 1 1] 三状态切换
  (:`Pressed`
    (if (== `_状态` 0)
      (bind _returnvalue (`|SpawnActorFromClass` "/Game/PP801_P3/Blueprints/Combines/weapon/Weapon_base.Weapon_base_C" (`KismetMathLibrary.MakeTransform` (0.0 0.0 0.0)) "Undefined" "OverrideRootScale" null null))
      (bind _output_get (set `self.装备好的武器` _returnvalue))
      (`self.K2_AttachToComponent` _output_get (`self.Mesh`) "WEAPON_R" "KeepRelative" "KeepRelative" "KeepRelative" true)
      (set `/Game/PP801_P3/Animations/Characters/NewAnimaBP/newMan_AnimBP1.状态` 1 _as_new_man_anim_bp1_0)
      (`KismetSystemLibrary.PrintString` "持枪")
      (elif (== `_状态` 1)
        (`self.K2_DestroyActor` _returnvalue)
        (bind _returnvalue_2 (`|SpawnActorFromClass` "/Game/PP801_P3/Blueprints/Combines/weapon/Weapon_base_2.Weapon_base_2_C" (`KismetMathLibrary.MakeTransform` (0.0 0.0 0.0)) "Undefined" "OverrideRootScale" null null))
        (`self.K2_AttachToComponent` _returnvalue_2 (`self.Mesh`) "WEAPON_R" "KeepRelative" "KeepRelative" "KeepRelative" true)
        (set `/Game/PP801_P3/Animations/Characters/NewAnimaBP/newMan_AnimBP1.状态` 2 _as_new_man_anim_bp1_0)
        (`|PlayMontage` (`self.Mesh`) "/Game/PP801_P3/Animations/Characters/RootMotion/Blade/Anim_B_Equip_Montage.Anim_B_Equip_Montage"
          (:`then`
            (`KismetSystemLibrary.PrintText` "持刀")))
        (else
          (`self.K2_DestroyActor` _returnvalue_2)
          (set `/Game/PP801_P3/Animations/Characters/NewAnimaBP/newMan_AnimBP1.状态` 0 _as_new_man_anim_bp1_0)
          (`KismetSystemLibrary.PrintString` "初始状态"))))))

(event `Key|E`
  (params (Key :type "Key Structure"))
  (bind `_装备好的武器` (`self.装备好的武器`))
  ;[1 1 1] 换弹
  (:`Pressed`
    (`|PlayMontage` (`self.Mesh`) "/Game/PP801_P3/Animations/Characters/NewAnimaBP/Reload_Pistol_Montage.Reload_Pistol_Montage" 1.0 0.0 "Defult"
      (:`OnCompleted`
        (set `/Game/PP801_P3/Blueprints/Combines/weapon/Weapon_base.BallutNum` (+ (`/Game/PP801_P3/Blueprints/Combines/weapon/Weapon_base.BallutNum` `_装备好的武器`) 5) `_装备好的武器`)))))

(event `Key|LeftControl`
  (params (Key :type "Key Structure"))
  (bind _returnvalue (`SkeletalMeshComponent.GetAnimInstance` (`self.Mesh`)))
  ;[1 1 1] R键蹲下行走
  (:`Pressed`
    (`/Engine/EditorBlueprintResources/StandardMacros.FlipFlop`
      (:`A`
        (bind _asnew_man_anim_bp1 (cast `/Game/PP801_P3/Animations/Characters/NewAnimaBP/newMan_AnimBP1` _returnvalue))
        (set `/Game/PP801_P3/Animations/Characters/NewAnimaBP/newMan_AnimBP1.GetDown?` true _asnew_man_anim_bp1)
        (set `self.是否可以设置最大速度` false))
      (:`B`
        (bind _asnew_man_anim_bp1_2 (cast `/Game/PP801_P3/Animations/Characters/NewAnimaBP/newMan_AnimBP1` _returnvalue))
        (set `/Game/PP801_P3/Animations/Characters/NewAnimaBP/newMan_AnimBP1.GetDown?` false _asnew_man_anim_bp1_2)
        (set `self.是否可以设置最大速度` true)))))

(event `Key|LeftMouseButton`
  (params (Key :type "Key Structure"))
  (bind _charactermovement (`self.CharacterMovement`))
  (bind `_状态` (`/Game/PP801_P3/Animations/Characters/NewAnimaBP/newMan_AnimBP1.状态` (`self.As New Man Anim BP1_0`)))
  ;[1 1 1] 攻击操作（包括空手攻击、近战武器攻击、枪攻击）
  (:`Pressed`
    (if (== `_状态` 1)
      (set `CharacterMovementComponent.MaxWalkSpeed` 150.0 (`self.CharacterMovement`))
      (`/Game/PP801_P3/Blueprints/Combines/weapon/Weapon_base.fire` (`self.装备好的武器`))
      (elif (== `_状态` 2)
        (set `CharacterMovementComponent.MaxWalkSpeed` 0.0 _charactermovement)
        (`|PlayMontage` (`self.Mesh`) "/Game/PP801_P3/Animations/Characters/RootMotion/Blade/Anim_B_Attack4_Montage.Anim_B_Attack4_Montage" 1.3 0.0 "Attack2"
          (:`OnCompleted`
            (set `CharacterMovementComponent.MaxWalkSpeed` 600.0 _charactermovement)))
        (else
          (`|PlayMontage` (`self.Mesh`) "/Game/PP801_P3/Animations/Characters/NewAnimaBP/Mage_Attack_04_Montage.Mage_Attack_04_Montage" 1.6))))))

(event `Key|LeftShift`
  (params (Key :type "Key Structure"))
  (bind _charactermovement (`self.CharacterMovement`))
  (bind `_是否可以设置最大速度` (`self.是否可以设置最大速度`))
  ;[1 1 1] Walk/Run
  (:`Pressed`
    (if `_是否可以设置最大速度`
      (set `CharacterMovementComponent.MaxWalkSpeed` 600.0 _charactermovement)))
  (:`Released`
    (if `_是否可以设置最大速度`
      (set `CharacterMovementComponent.MaxWalkSpeed` 150.0 _charactermovement))))

(event `Key|E`
  (params (Key :type "Key Structure"))
  (bind _mesh (`self.Mesh`))
  ;[1 1 1] 攻击模板
  (:`Pressed`
    (bind _asnew_man_anim_bp1 (cast `/Game/PP801_P3/Animations/Characters/NewAnimaBP/newMan_AnimBP1` (`SkeletalMeshComponent.GetAnimInstance` (`self.Mesh`))))
    (if (`/Game/PP801_P3/Animations/Characters/NewAnimaBP/newMan_AnimBP1.拿枪` _asnew_man_anim_bp1)
      (`|PlayMontage` _mesh)
      (elif (`/Game/PP801_P3/Animations/Characters/NewAnimaBP/newMan_AnimBP1.拿刀` _asnew_man_anim_bp1)
        (`|PlayMontage` _mesh "/Game/PP801_P3/Animations/Characters/RootMotion/Blade/Anim_B_Attack4_Montage.Anim_B_Attack4_Montage"
          (:`OnCompleted`
            (`KismetSystemLibrary.PrintString` "finish"))
          (:`OnInterrupted`
            (`KismetSystemLibrary.PrintString` "fail")))
        (else
          (`|PlayMontage` _mesh))))))

(fn `UserConstructionScript`
  (`parent.UserConstructionScript`))